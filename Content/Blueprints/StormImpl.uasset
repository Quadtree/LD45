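; Storm controller actor that pushes its StormLevel value into the sky's material.
; On BeginPlay it finds static mesh actors tagged "Sky", gives each a dynamic instance of its first material and stores it in a single SkyMaterial variable.
; Every Tick writes StormLevel to that stored instance's scalar parameter, so only the last sky mesh processed receives updates.
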(event `self.ReceiveBeginPlay`
  (bind _outactors (`GameplayStatics.GetAllActorsWithTag` "Sky"))
  (for _array_element _outactors
    (bind _asstatic_mesh_actor (cast `StaticMeshActor` _array_element))
    (bind _staticmeshcomponent (`StaticMeshActor.StaticMeshComponent` _asstatic_mesh_actor))
    (bind _returnvalue (`PrimitiveComponent.CreateDynamicMaterialInstance` _staticmeshcomponent 0 (`PrimitiveComponent.GetMaterial` _staticmeshcomponent 0) "None"))
    (bind _output_get (set `self.SkyMaterial` _returnvalue))
    (`PrimitiveComponent.SetMaterial` (`StaticMeshActor.StaticMeshComponent` _asstatic_mesh_actor) 0 _output_get)))

(event `self.ReceiveTick`
  (params (DeltaSeconds :type "Float (single-precision)"))
  (`MaterialInstanceDynamic.SetScalarParameterValue` (`self.SkyMaterial`) "StormLevel" (`self.StormLevel`)))

(fn `UserConstructionScript`)