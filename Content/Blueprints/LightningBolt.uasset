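; Lightning bolt actor that plunges downward in an erratic path and heats flammable actors it strikes.
; Redirect gives the physics Sphere a fixed high downward velocity with random sideways drift, at BeginPlay and randomly about ten times per second via a delta-time-scaled Tick check.
; On hitting an actor with a FlammableComponent, it sets that component's Temperature very high and destroys itself; other hits leave it alive.
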(event `self.ReceiveBeginPlay`
  (`self.Redirect`))

(event `self.ReceiveTick`
  (params (DeltaSeconds :type "Float (single-precision)"))
  (if (< (`KismetMathLibrary.RandomFloat`) (* DeltaSeconds 10.0))
    (`self.Redirect`)))

(event `self.ReceiveHit`
  (params (MyComp :type "PrimitiveComponent Object Reference") (Other :type "Actor Object Reference") (OtherComp :type "PrimitiveComponent Object Reference") (bSelfMoved :type Boolean) (HitLocation :type "Vector Structure") (HitNormal :type "Vector Structure") (NormalImpulse :type "Vector Structure") (Hit :type "HitResult Structure (by ref)"))
  (bind _returnvalue (`self.GetComponentByClass` Other "/Script/LD45.FlammableComponent"))
  (`/Engine/EditorBlueprintResources/StandardMacros.IsValid` _returnvalue
    (:`Is Valid`
      (set `FlammableComponent.Temperature` 1000.0 _returnvalue)
      (`self.K2_DestroyActor`))))

(fn `Redirect`
  (`PrimitiveComponent.SetPhysicsLinearVelocity` (`self.Sphere`) (`KismetMathLibrary.MakeVector` (`KismetMathLibrary.RandomFloatInRange` -200.0 200.0) (`KismetMathLibrary.RandomFloatInRange` -200.0 200.0) (`KismetMathLibrary.RandomFloatInRange` -70000.0 -70000.0)) false "None"))

(fn `UserConstructionScript`)