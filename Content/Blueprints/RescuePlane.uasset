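; RescuePlane is an actor that flies over the terrain and triggers the win when it detects a hot enough flammable object.
; It starts behind and above the Terrain5_Blueprint's highest point, moves a fixed step along +X each tick, and destroys itself past an X limit.
; A per-tick sphere overlap checks FlammableComponent temperatures, adding a WinScreen widget for every hit, with no guard against repeats.
; Movement is frame-rate dependent.
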(event `self.ReceiveBeginPlay`
  (bind _returnvalue (`GameplayStatics.GetActorOfClass` "/Game/Blueprints/Terrain5_Blueprint.Terrain5_Blueprint_C"))
  (`self.K2_SetActorLocation` (+ (`Terrain.HighestPoint` _returnvalue) (-40000.0 0.0 3000.0))))

(event `self.ReceiveTick`
  (params (DeltaSeconds :type "Float (single-precision)"))
  (if (> (.x (`self.K2_GetActorLocation`)) 50000.0)
    (`self.K2_DestroyActor`)
    (else
      (`self.K2_SetActorLocation` (+ (`self.K2_GetActorLocation`) (`KismetMathLibrary.MakeVector` 30.0)))
      (bind _outactors (`KismetSystemLibrary.SphereOverlapActors` (`self.K2_GetActorLocation`) 3400.0 (`|MakeArray` "ObjectTypeQuery1" "ObjectTypeQuery2" "ObjectTypeQuery4" :!type "EObjectTypeQuery Enum")))
      (for _array_element _outactors
        (bind _returnvalue (`self.GetComponentByClass` _array_element "/Script/LD45.FlammableComponent"))
        (`/Engine/EditorBlueprintResources/StandardMacros.IsValid` _returnvalue
          (:`Is Valid`
            (if (> (`FlammableComponent.Temperature` _returnvalue) 200.0)
              (`KismetSystemLibrary.PrintString` "YOU WIN")
              (bind _returnvalue_2 (`|CreateWidget` "/Game/UI/WinScreen.WinScreen_C"))
              (`UserWidget.AddToViewport` _returnvalue_2 0))))))))

(fn `UserConstructionScript`)