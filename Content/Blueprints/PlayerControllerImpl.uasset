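; Player controller Blueprint that handles menu confirmation and storm debug cheats through direct key bindings.
; Space finds any top-level title, win and lose screen widgets by class, starting the game from the title and restarting it from the end screens.
; When cheats are enabled, the bracket keys look up the StormImpl actor to start a storm or trigger wind shear.
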(event `Key|SpaceBar` :consume false :paused true
  (params (Key :type "Key Structure"))
  (:`Pressed`
    (bind _foundwidgets (`WidgetBlueprintLibrary.GetAllWidgetsOfClass` "/Game/UI/TitleScreen.TitleScreen_C"))
    (for _array_element _foundwidgets
      (`/Game/UI/TitleScreen.StartGame` _array_element))
    (bind _foundwidgets_2 (`WidgetBlueprintLibrary.GetAllWidgetsOfClass` "/Game/UI/WinScreen.WinScreen_C"))
    (for _array_element_2 _foundwidgets_2
      (`/Game/UI/WinScreen.RestartGame` _array_element_2))
    (bind _foundwidgets_3 (`WidgetBlueprintLibrary.GetAllWidgetsOfClass` "/Game/UI/LoseScreen.LoseScreen_C"))
    (for _array_element_3 _foundwidgets_3
      (`/Game/UI/LoseScreen.RestartGame` _array_element_3))))

(event `Key|RightBracket`
  (params (Key :type "Key Structure"))
  (:`Pressed`
    (if (`LD45GameMode.GetCheatsEnabled`)
      (bind _returnvalue (`GameplayStatics.GetActorOfClass` "/Game/Blueprints/StormImpl.StormImpl_C"))
      (`Storm.StartStorm` _returnvalue 1.0))))

(event `Key|LeftBracket`
  (params (Key :type "Key Structure"))
  (:`Pressed`
    (if (`LD45GameMode.GetCheatsEnabled`)
      (bind _returnvalue (`GameplayStatics.GetActorOfClass` "/Game/Blueprints/StormImpl.StormImpl_C"))
      (`Storm.WindShear` _returnvalue))))

(fn `UserConstructionScript`)